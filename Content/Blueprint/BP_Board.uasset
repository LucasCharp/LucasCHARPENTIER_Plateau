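; BP_Board is the board actor that holds a list of cell actors and provides their positions to the game.
; On BeginPlay it casts the game mode to BP_Gamemode and stores itself there as BoardRef.
; GetCellPositionByNumber looks up a cell by index and returns its X, Y and Z location, with Z raised by a small fixed offset.
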(event `self.ReceiveBeginPlay`
  (bind _asbp_gamemode (cast `/Game/Blueprint/BP_Gamemode` (`GameplayStatics.GetGameMode`)))
  (bind _output_get (set `self.As BP Gamemode` _asbp_gamemode))
  (set `/Game/Blueprint/BP_Gamemode.BoardRef` self _output_get))

(fn `GetCellPositionByNumber`
  (params (CellIndex :type Integer))
  (returns (CellLocation :type "Vector Structure"))
  (bind _returnvalue (`self.GetTransform` (`|GetArrayItem` (`self.CellList`) CellIndex)))
  (return (`KismetMathLibrary.MakeVector` (.x (.location _returnvalue)) (.y (.location _returnvalue)) (+ (.z (.location _returnvalue)) 20.0))))

(fn `UserConstructionScript`)