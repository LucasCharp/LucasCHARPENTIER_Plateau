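; BP_Dice is a dice roller that rolls once when play begins.
; DiceRoll sums a random integer between DiceValueMin and DiceValueMax for each of DiceNumber dice into DiceResult.
; The total is printed to screen with PrintString; overlap and tick events are unused.
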(event `self.ReceiveBeginPlay`
  (`self.DiceRoll`))

(fn `DiceRoll`
  (set `self.DiceResult` 0)
  (for _ (range 1 (+ (`self.Dice Number`) 1))
    (bind _output_get (set `self.DiceResult` (+ (`self.DiceResult`) (`KismetMathLibrary.RandomIntegerInRange` (`self.DiceValueMin`) (`self.DiceValueMax`))))))
  (`KismetSystemLibrary.PrintString` (`KismetStringLibrary.Conv_IntToString` _output_get))
  (return))

(fn `UserConstructionScript`)