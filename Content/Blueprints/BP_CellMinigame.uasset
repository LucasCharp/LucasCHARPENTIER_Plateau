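; BP_CellMinigame is a cell that sends play into a randomly chosen minigame when its Action is triggered.
; It caches BP_GameInstance on BeginPlay, and its Action override runs the parent logic, then randomly opens either the Memory or the Chase level.
; Only the Memory branch stores the triggering player's ID in the game instance as the solo minigame player before changing level.
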(event `self.ReceiveBeginPlay`
  (`parent.ReceiveBeginPlay`)
  (bind _asbp_game_instance (cast `/Game/Blueprints/BP_GameInstance` (`GameplayStatics.GetGameInstance`)))
  (set `self.As BP Game Instance_0` _asbp_game_instance))

(fn `Action`
  (params (PlayerId :type Integer))
  (`parent.Action` PlayerId)
  (bind _output_get (set `self.MiniGame` (`KismetMathLibrary.RandomInteger` 2)))
  (switch `int` _output_get
    (:`0`
      (set `/Game/Blueprints/BP_GameInstance.playerIdForSoloMinigame` PlayerId (`self.As BP Game Instance_0`))
      (`GameplayStatics.OpenLevelBySoftObjectPtr` "/Game/Maps/LV_Memorytrue.LV_Memorytrue"))
    (:`1`
      (`GameplayStatics.OpenLevelBySoftObjectPtr` "/Game/Maps/LV_Chase.LV_Chase"))))

(fn `UserConstructionScript`
  (`parent.UserConstructionScript`))