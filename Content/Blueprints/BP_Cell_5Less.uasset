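; BP_Cell_5Less is a penalty cell that takes points from a player, labeled "-5 points".
; It sets its effect text on BeginPlay, then runs the parent's BeginPlay.
; Its Action override calls the parent, subtracts ScoreLess from that player's score through the game instance, refreshes the score display and returns CanChangePlayer.
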(event `self.ReceiveBeginPlay`
  (set `self.textEffect` "-5 points")
  (`parent.ReceiveBeginPlay`))

(fn `Action`
  (params (PlayerId :type Integer))
  (returns (changePlayer :type Boolean))
  (bind _as_bp_game_instance (`self.As BP Game Instance`))
  (`parent.Action` PlayerId)
  (bind _playerscore (`/Game/Blueprints/BP_GameInstance.GetPlayerScoreByPlayerId` (`self.As BP Game Instance`) PlayerId))
  (`/Game/Blueprints/BP_GameInstance.SetPlayerScoreByPlayerId` _as_bp_game_instance PlayerId (- _playerscore (`self.ScoreLess`)))
  (`/Game/Blueprints/BP_GameInstance.ShowPlayerScoreByPlayerId` _as_bp_game_instance PlayerId)
  (return (`self.canChangePlayer`)))

(fn `UserConstructionScript`
  (`parent.UserConstructionScript`))