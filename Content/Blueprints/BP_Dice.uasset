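; BP_Dice is a Blueprint that rolls dice and shows the total on screen.
; RollDice sums DiceNumber random rolls, each from 1 to DiceType, into ActualDiceResult.
; It then creates a WB_Dice widget, adds it to the viewport and calls StartAnim with the result.
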(fn `RollDice`
  (set `self.ActualDiceResult` 0)
  (for _ (range 1 (+ (`self.DiceNumber`) 1))
    (bind _output_get (set `self.ActualDiceResult` (+ (`self.ActualDiceResult`) (`KismetMathLibrary.RandomIntegerInRange` 1 (`self.DiceType`))))))
  (bind _returnvalue (`|CreateWidget` "/Game/Widget/WB_Dice.WB_Dice_C"))
  (bind _output_get_2 (set `self.WidgetDice` _returnvalue))
  (`UserWidget.AddToViewport` _output_get_2 0)
  (`/Game/Widget/WB_Dice.StartAnim` _output_get_2 _output_get)
  (return))

(fn `UserConstructionScript`)