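; Game mode for a memory matching game with cards and chests, tracking a score.
; Each click handler stores the first picked actor, then compares it with the second: cards by Color, chests by their contents.
; A match adds a point and destroys both actors; a mismatch toggles or closes both back and clears the stored pick.
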(event `self.ReceiveBeginPlay`)

(fn `OnCardClicked`
  (params (Card :type "/Game/Blueprints/Cards/BP_Card Object Reference"))
  (if (`KismetSystemLibrary.IsValid` (`self.PrevCard`))
    (if (`|EnumEquality` (`/Game/Blueprints/Cards/BP_Card.Color` Card) (`/Game/Blueprints/Cards/BP_Card.Color` (`self.PrevCard`)))
      (`/Engine/EditorBlueprintResources/StandardMacros.IncrementInt` (`self.Score`)
        (:`  `
          (`self.K2_DestroyActor` Card)
          (`self.K2_DestroyActor` (`self.PrevCard`))))
      (else
        (`/Game/Blueprints/Cards/BP_Card.Toggle Card` Card)
        (`/Game/Blueprints/Cards/BP_Card.Toggle Card` (`self.PrevCard`))))
    (set `self.PrevCard` null)
    (else
      (set `self.PrevCard` Card))))

(fn `OnChestClicked`
  (params (Chest :type "/Game/Blueprints/Chest/BP_Chest Object Reference"))
  (if (`KismetSystemLibrary.IsValid` (`self.PrevChest`))
    (if (`|EnumEquality` (`/Game/Blueprints/Chest/BP_Chest.ChestContains` Chest) (`/Game/Blueprints/Chest/BP_Chest.ChestContains` (`self.PrevChest`)))
      (`/Engine/EditorBlueprintResources/StandardMacros.IncrementInt` (`self.Score`)
        (:`  `
          (`self.K2_DestroyActor` Chest)
          (`self.K2_DestroyActor` (`self.PrevChest`))))
      (else
        (`/Game/Blueprints/Chest/BP_Chest.Open/Close` (`self.PrevChest`))
        (`/Game/Blueprints/Chest/BP_Chest.Open/Close` Chest)))
    (set `self.PrevChest` null)
    (else
      (set `self.PrevChest` Chest))))

(fn `UserConstructionScript`)