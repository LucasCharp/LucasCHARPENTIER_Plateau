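; BP_Player is the player Blueprint that drives a dice-based game through two debug keys.
; On BeginPlay it caches BP_GameMode, whose game instance holds the GameHasBeenSet flag.
; P calls SetGame on the game mode while the flag is false, and E calls RollADiceAndMove once it is true.
; All game logic is delegated to the game mode.
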(event EventBeginPlay
  (bind _asbp_game_mode (Utilities|Casting|CastToBP_GameMode (Game|GetGameMode)))
  (Variables|Default|SetAs%20BP%20Game%20Mode _asbp_game_mode))

(event Collision|EventActorBeginOverlap
  (params (OtherActor :type Actor%20Object%20Reference)))

(event EventTick
  (params (DeltaSeconds :type Float%20%28single-precision%29)))

(event Input|KeyboardEvents|DebugKeyE
  (params (Key :type Key%20Structure :default "None") (ActionValue :type Input%20Action%20Value%20Structure))
  (bind _as_bp_game_mode (Variables|Default|GetAs%20BP%20Game%20Mode))
  (:Pressed
    (if (Variables|/Game/Blueprints/BP_GameInstance.BP_GameInstance_C|GetgameHasBeenSet? (Variables|/Game/Blueprints/BP_GameMode.BP_GameMode_C|GetAs%20BP%20Game%20Instance _as_bp_game_mode))
      (Default|RollADiceandMove _as_bp_game_mode))))

(event Input|KeyboardEvents|DebugKeyP
  (params (Key :type Key%20Structure :default "None") (ActionValue :type Input%20Action%20Value%20Structure))
  (bind _as_bp_game_mode (Variables|Default|GetAs%20BP%20Game%20Mode))
  (bind _as_bp_game_instance (Variables|/Game/Blueprints/BP_GameMode.BP_GameMode_C|GetAs%20BP%20Game%20Instance _as_bp_game_mode))
  (:Pressed
    (if (not (Variables|/Game/Blueprints/BP_GameInstance.BP_GameInstance_C|GetgameHasBeenSet? _as_bp_game_instance))
      (Default|SetGame _as_bp_game_mode _as_bp_game_instance))))

(fn ConstructionScript)