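; BP_Card is a clickable card actor for a memory game, with a color that sets the material on its Verso mesh at construction.
; Clicking a clickable card calls ToggleCard, waits a second, then reports the card to BP_GamemodeMemory, cached on BeginPlay.
; ToggleCard inverts IsClickable and flips the root between 0 and 180 degrees of roll, so a turned card ignores further clicks.
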(event `self.ReceiveBeginPlay`
  (bind _asbp_gamemode_memory (cast `/Game/Blueprints/BP_GamemodeMemory` (`GameplayStatics.GetGameMode`)))
  (set `self.As BP Gamemode Memory` _asbp_gamemode_memory))

(event `self.ReceiveActorOnClicked`
  (params (ButtonPressed :type "Key Structure"))
  (if (`self.isClickable`)
    (`self.Toggle Card`)
    (`KismetSystemLibrary.Delay` 1.0)
    (`/Game/Blueprints/BP_GamemodeMemory.OnCardClicked` (`self.As BP Gamemode Memory`) self)))

(fn `ChangeCardColor`
  (bind _verso (`self.Verso`))
  (switch `/Game/Blueprints/Cards/E_CardColor` (`self.Color`)
    (:`NewEnumerator1`
      (`PrimitiveComponent.SetMaterial` _verso 0 "/Game/Material/MI_YellowCard.MI_YellowCard"))
    (:`NewEnumerator2`
      (`PrimitiveComponent.SetMaterial` _verso 0 "/Game/Material/MI_RedCard.MI_RedCard"))
    (:`NewEnumerator3`
      (`PrimitiveComponent.SetMaterial` _verso 0 "/Game/Material/MI_BlueCard.MI_BlueCard"))
    (:`NewEnumerator4`
      (`PrimitiveComponent.SetMaterial` _verso 0 "/Game/Material/MI_GreenCard.MI_GreenCard"))))

(fn `Toggle Card`
  (bind _defaultsceneroot (`self.DefaultSceneRoot`))
  (bind _returnvalue_roll (`KismetMathLibrary.BreakRotator` (`SceneComponent.K2_GetComponentRotation` (`self.DefaultSceneRoot`))))
  (set `self.isClickable` (not (`self.isClickable`)))
  (if (== _returnvalue_roll 0.0)
    (`SceneComponent.K2_SetRelativeRotation` _defaultsceneroot (`KismetMathLibrary.MakeRotator` 180.0) false false)
    (else
      (`SceneComponent.K2_SetRelativeRotation` _defaultsceneroot (`KismetMathLibrary.MakeRotator` 0.0) false false))))

(fn `UserConstructionScript`
  (`self.ChangeCardColor`))