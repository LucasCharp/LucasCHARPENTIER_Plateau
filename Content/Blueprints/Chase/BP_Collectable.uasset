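; Collectable actor for the Chase game mode that awards score to players who touch it.
; It caches the Chase game mode on BeginPlay, then on box overlap checks whether the other actor is in the mode's player collect list.
; For a match, it updates the score by player ID through the game mode and writes the result to that player's score widget text.
; The collectable neither destroys nor hides itself here.
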(event `self.ReceiveBeginPlay`
  (bind _asbp_gamemode_chase (cast `/Game/Blueprints/Chase/BP_GamemodeChase` (`GameplayStatics.GetGameMode`)))
  (set `self.As BP Gamemode Chase` _asbp_gamemode_chase))

(event `self.Box.OnComponentBeginOverlap`
  (params (OverlappedComponent :type "PrimitiveComponent Object Reference") (OtherActor :type "Actor Object Reference") (OtherComp :type "PrimitiveComponent Object Reference") (OtherBodyIndex :type Integer) (bFromSweep :type Boolean) (SweepResult :type "HitResult Structure (by ref)"))
  (bind _as_bp_gamemode_chase (`self.As BP Gamemode Chase`))
  (for _array_element (`GamemodeChase.PlayerCollectList` (`self.As BP Gamemode Chase`))
    (if (== _array_element OtherActor)
      (bind _playerid (`PlayerCollect.playerID` _array_element))
      ;[1 0 0] !IMPORTANT! Replacer ce node à chaque redémarrage. Peut-etre pas en fait mais je le laisse dans le doute
      (bind _returnvalue (`GamemodeChase.SetScoreByPlayerId` _as_bp_gamemode_chase _playerid))
      (`TextBlock.SetText` (`|GetArrayItem` (`/Game/Widget/WB_ChaseScore.ChasePlayerScore` (`/Game/Blueprints/Chase/BP_GamemodeChase.ChaseScoreWidget` _as_bp_gamemode_chase)) _playerid) (`KismetTextLibrary.Conv_IntToText` _returnvalue)))))

(fn `UserConstructionScript`)