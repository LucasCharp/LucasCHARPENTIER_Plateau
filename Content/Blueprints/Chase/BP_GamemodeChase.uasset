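; Game mode for the Chase minigame, running it from the explanation screen through to the winner screen.
; StartChase swaps the explanation for the score HUD, spawns a player at a spawn point for each player in the game instance, triggers possession, then starts the round after a short delay.
; Tick updates the timer text and shows the winner once when time ends.
; A helper increments a player's score by ID.
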(event `self.ReceiveBeginPlay`
  (bind _asbp_game_instance (cast `/Game/Blueprints/BP_GameInstance` (`GameplayStatics.GetGameInstance`)))
  (set `self.As BP Game Instance` _asbp_game_instance)
  (bind _aspc_player_chase (cast `/Game/Blueprints/Chase/PC_PlayerChase` (`GameplayStatics.GetPlayerController` 0)))
  (bind _output_get (set `self.As PC Player Chase` _aspc_player_chase))
  (set `PlayerController.bShowMouseCursor` true _output_get)
  (bind _returnvalue (`|CreateWidget` "/Game/Widget/WB_ExplicationChase.WB_ExplicationChase_C"))
  (bind _output_get_2 (set `self.ExplicationChaseWidget` _returnvalue))
  (`UserWidget.AddToViewport` _output_get_2 0))

(event `self.ReceiveTick`
  (params (DeltaSeconds :type "Float (single-precision)"))
  (if (`self.realChaseHasStarted`)
    (`TextBlock.SetText` (`/Game/Widget/WB_ChaseScore.TimerLeft` (`self.ChaseScoreWidget`)) (`KismetTextLibrary.Conv_DoubleToText` (`self.Time`) "HalfToEven"))
    (if (`self.timeHasEnd`)
      (`/Engine/EditorBlueprintResources/StandardMacros.DoOnce` false
        (:`Completed`
          (bind _returnvalue (`|CreateWidget` "/Game/Widget/WB_FinChase.WB_FinChase_C"))
          (`UserWidget.AddToViewport` _returnvalue 0)
          (`Widget.RemoveFromParent` (`self.ChaseScoreWidget`))
          (set `PlayerController.bShowMouseCursor` true (`self.As PC Player Chase`))
          (`/Game/Widget/WB_FinChase.ShowChaseWinner` _returnvalue (`self.winnerId`) (`self.winnerScore`)))))))

(event `StartChase`
  (`Widget.RemoveFromParent` (`self.ExplicationChaseWidget`))
  (set `PlayerController.bShowMouseCursor` false (`self.As PC Player Chase`))
  (bind _returnvalue (`|CreateWidget` "/Game/Widget/WB_ChaseScore.WB_ChaseScore_C"))
  (`UserWidget.AddToViewport` _returnvalue 0)
  (set `self.ChaseScoreWidget` _returnvalue)
  (for _index (range (`/Game/Blueprints/BP_GameInstance.NumberOfPlayers` (`self.As BP Game Instance`)))
    (bind _returnvalue_2 (`|SpawnActorFromClass` "/Game/Blueprints/Chase/BP_PlayerChase.BP_PlayerChase_C" (`self.GetTransform` (`|GetArrayItem` (`/Game/Blueprints/Chase/BP_SpawnPoints.Spawner` (`self.SpawnPointsRef`)) _index)) "Undefined" "MultiplyWithRoot" null null))
    (`KismetArrayLibrary.Array_Set` (`self.PlayerCollectList`) _index _returnvalue_2 true)
    (`Widget.SetVisibility` (`|GetArrayItem` (`/Game/Widget/WB_ChaseScore.ChasePlayerScore` (`self.ChaseScoreWidget`)) _index) "Visible")
    (`Widget.SetVisibility` (`|GetArrayItem` (`/Game/Widget/WB_ChaseScore.ChaseScoreWords` (`self.ChaseScoreWidget`)) _index) "Visible"))
  (`/Game/Blueprints/Chase/PC_PlayerChase.PossessPlayer` (`self.As PC Player Chase`))
  (`KismetSystemLibrary.Delay` 0.8)
  (set `self.realChaseHasStarted` true))

(fn `SetPlayerScoreByPlayerId`
  (params (PlayerId :type Integer))
  (bind _result (`/Engine/EditorBlueprintResources/StandardMacros.IncrementInt` (`PlayerCollect.chaseScore` (`|GetArrayItem` (`self.PlayerCollectList`) PlayerId)))
    (:`  `
      (`KismetSystemLibrary.PrintString` (`KismetStringLibrary.Conv_IntToString` _result)))))

(fn `UserConstructionScript`)