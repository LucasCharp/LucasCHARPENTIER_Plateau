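; Clickable chest for a memory game, showing one of several treasure types such as coins, crystals, maps or weapons.
; The construction script sets the Plane material from ChestContains.
; Clicking an openable chest toggles IsOpenable, snaps Cube6 between two rotations based on its current world roll, then notifies BP_GamemodeMemory after a short delay.
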(event `self.ReceiveBeginPlay`
  (bind _asbp_gamemode_memory (cast `/Game/Blueprints/BP_GamemodeMemory` (`GameplayStatics.GetGameMode`)))
  (set `self.As BP Gamemode Memory` _asbp_gamemode_memory)
  (set `self.RCubeComp` (`self.Cube6`)))

(event `self.ReceiveActorOnClicked`
  (params (ButtonPressed :type "Key Structure"))
  (if (`self.bIsOpenable`)
    (`self.OpenClose`)
    (`KismetSystemLibrary.Delay` 1.0)
    (`/Game/Blueprints/BP_GamemodeMemory.OnChestClicked` (`self.As BP Gamemode Memory`) self)))

(fn `ChangeChestType`
  (bind _plane (`self.Plane`))
  (switch `/Game/Blueprints/Chest/E_Chest` (`self.ChestContains`)
    (:`NewEnumerator0`
      (`PrimitiveComponent.SetMaterial` _plane 0 "/Game/Blueprints/Chest/ChestImages/M_Coins.M_Coins"))
    (:`NewEnumerator1`
      (`PrimitiveComponent.SetMaterial` _plane 0 "/Game/Blueprints/Chest/ChestImages/M_RedCrystal.M_RedCrystal"))
    (:`NewEnumerator2`
      (`PrimitiveComponent.SetMaterial` _plane 0 "/Game/Blueprints/Chest/ChestImages/M_GreenCrystal.M_GreenCrystal"))
    (:`NewEnumerator3`
      (`PrimitiveComponent.SetMaterial` _plane 0 "/Game/Blueprints/Chest/ChestImages/M_BlueCrystal.M_BlueCrystal"))
    (:`NewEnumerator4`
      (`PrimitiveComponent.SetMaterial` _plane 0 "/Game/Blueprints/Chest/ChestImages/M_YellowCrystal.M_YellowCrystal"))
    (:`NewEnumerator5`
      (`PrimitiveComponent.SetMaterial` _plane 0 "/Game/Blueprints/Chest/ChestImages/M_PurpleCrystals.M_PurpleCrystals"))
    (:`NewEnumerator6`
      (`PrimitiveComponent.SetMaterial` _plane 0 "/Game/Blueprints/Chest/ChestImages/M_TreasureMaps.M_TreasureMaps"))
    (:`NewEnumerator7`
      (`PrimitiveComponent.SetMaterial` _plane 0 "/Game/Blueprints/Chest/ChestImages/M_SwordStack.M_SwordStack"))
    (:`NewEnumerator8`
      (`PrimitiveComponent.SetMaterial` _plane 0 "/Game/Blueprints/Chest/ChestImages/M_PirateGuns.M_PirateGuns"))
    (:`NewEnumerator9`
      (`PrimitiveComponent.SetMaterial` _plane 0 "/Game/Blueprints/Chest/ChestImages/M_Bottles.M_Bottles"))))

(fn `Open/Close`
  (bind _cube6 (`self.Cube6`))
  (bind _returnvalue_roll (`KismetMathLibrary.BreakRotator` (`SceneComponent.K2_GetComponentRotation` (`self.Cube6`))))
  (set `self.isOpenable` (not (`self.isOpenable`)))
  (if (< _returnvalue_roll 1.0)
    (`SceneComponent.K2_SetRelativeRotation` _cube6 (`KismetMathLibrary.MakeRotator` 0.0 90.0) false false)
    (else
      (`SceneComponent.K2_SetRelativeRotation` _cube6 (`KismetMathLibrary.MakeRotator` 0.0) false false))))

(fn `UserConstructionScript`
  (`self.ChangeChestType`))