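; BP_Dice is a Blueprint that simulates rolling a configurable number of dice and totalling the result.
; Its DiceRoll function resets DiceResult, adds a random integer between DiceValueMin and DiceValueMax once per die, then prints the sum.
; The event graph and construction script are empty, so nothing in this Blueprint calls the roll itself.
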(event `self.ReceiveBeginPlay`)

(fn `DiceRoll`
  (set `self.DiceResult` 0)
  (for _ (range 1 (+ (`self.Dice Number`) 1))
    (bind _output_get (set `self.DiceResult` (+ (`self.DiceResult`) (`KismetMathLibrary.RandomIntegerInRange` (`self.DiceValueMin`) (`self.DiceValueMax`))))))
  (`KismetSystemLibrary.PrintString` (`KismetStringLibrary.Conv_IntToString` _output_get) true true (struct :`G` 0.66 :`B` 1.0 :`A` 1.0) 4.0)
  (return))

(fn `UserConstructionScript`)