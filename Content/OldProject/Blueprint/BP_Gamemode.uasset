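; Game mode for a dice-driven board game that spawns pawns, moves them and ends the match.
; On BeginPlay it reads players from BP_Gameinstance, spawns each pawn at its saved cell on BP_Board and creates a BP_Dice.
; RollADiceAndMove plays a full round, rolling for each player, saving the new cell and moving the pawn.
; Reaching the last cell clamps the move, flags the game finished, shows WB_Victoire and stops the round.
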(event `self.ReceiveBeginPlay`
  (bind _asbp_gameinstance (cast `/Game/OldProject/Blueprint/BP_Gameinstance` (`GameplayStatics.GetGameInstance`)))
  (bind _output_get (set `self.As BP Gameinstance` _asbp_gameinstance))
  ;[1 1 1] Donne au jeu le nombre de players
  (bind _output_get_2 (set `/Game/OldProject/Blueprint/BP_Gameinstance.NumberOfPlayer` (`KismetArrayLibrary.Array_Length` (`/Game/OldProject/Blueprint/BP_Gameinstance.PlayerList` _output_get)) _output_get))
  ;[1 1 1] Fait spawn des joueurs jusqu'à ce qu'ils soient tous sur le plateau
  (for _index (range _output_get_2)
    (`self.SpawnPion` _index))
  ;[1 1 1] Set le nombre de case sur le plateau
  (set `self.NumberOfBoardCells` (`KismetArrayLibrary.Array_Length` (`/Game/OldProject/Blueprint/BP_Board.CellList` (`self.BoardRef`))))
  (bind _returnvalue (`|SpawnActorFromClass` "/Game/OldProject/Blueprint/BP_Dice.BP_Dice_C" (`KismetMathLibrary.MakeTransform` (0.0 0.0 0.0)) "Undefined" "MultiplyWithRoot" null null))
  (set `self.Dice` _returnvalue))

(fn `RollADiceAndMove`
  (bind _dice (`self.Dice`))
  (bind _as_bp_gameinstance (`self.As BP Gameinstance`))
  (bind _returnvalue (- (`self.NumberOfBoardCells`) 1))
  ;[1 1 1] Ça va lancer un dé et faire avancer le joueur. Ensuite, ça va faire un nouveau lancer pour le second joueur et ainsi de suite selon le nombre total de joueur
  (for _index (range (`/Game/OldProject/Blueprint/BP_Gameinstance.NumberOfPlayer` _as_bp_gameinstance))
    (`/Game/OldProject/Blueprint/BP_Dice.DiceRoll` _dice)
    (bind _playercellnumber (`/Game/OldProject/Blueprint/BP_Gameinstance.GetPlayerCellNumberByPlayerId` _as_bp_gameinstance _index))
    (bind _returnvalue_2 (+ _playercellnumber (`/Game/OldProject/Blueprint/BP_Dice.DiceResult` _dice)))
    (`/Game/OldProject/Blueprint/BP_Gameinstance.SetPLayerCellNumberByPlayerId` _as_bp_gameinstance _index _returnvalue_2)
    ;[1 1 1] Print en rouge le numéro de la case où il a atterit
    (`KismetSystemLibrary.PrintString` (`KismetStringLibrary.Concat_StrStr` "Player " (`KismetStringLibrary.Conv_IntToString` _index) " : Cell Number " (`KismetStringLibrary.Conv_IntToString` _returnvalue_2)) true true (struct :`R` 1.0 :`G` 0.015318 :`A` 1.0) 4.0)
    (if (>= _returnvalue_2 _returnvalue)
      (set `self.ActualCell` _returnvalue)
      (set `/Game/OldProject/Blueprint/BP_Gameinstance.isFinish` true (`self.As BP Gameinstance`))
      (else
        (set `self.ActualCell` _returnvalue_2)))
    ;[1 1 1] Il continue d'avancer normalement.
    (bind _celllocation (`/Game/OldProject/Blueprint/BP_Board.GetCellPositionByNumber` (`self.BoardRef`) (`self.ActualCell`)))
    (`/Game/OldProject/Blueprint/BP_Pion.MoveToNewCell` (`|GetArrayItem` (`self.PionPlayer`) _index) _celllocation)
    (set `self.ActualPlayerId` (mod (+ (`self.ActualPlayerId`) 1) 2))
    ;[1 1 1] FIN
    (if (`/Game/OldProject/Blueprint/BP_Gameinstance.isFinish` (`self.As BP Gameinstance`))
      (bind _returnvalue_3 (`|CreateWidget` "/Game/Widget/WB_Victoire.WB_Victoire_C"))
      (`UserWidget.AddToViewport` _returnvalue_3 0)
      (set `PlayerController.bShowMouseCursor` true (`GameplayStatics.GetPlayerController` 0))
      (break))))

(fn `SpawnPion`
  (params (PlayerId :type Integer))
  (bind _as_bp_gameinstance (`self.As BP Gameinstance`))
  (bind _returnvalue (`GameplayStatics.GetActorOfClass` "/Game/OldProject/Blueprint/BP_Board.BP_Board_C"))
  (bind _output_get (set `self.BoardRef` _returnvalue))
  (bind _playercellnumber (`/Game/OldProject/Blueprint/BP_Gameinstance.GetPlayerCellNumberByPlayerId` _as_bp_gameinstance PlayerId))
  (bind _celllocation (`/Game/OldProject/Blueprint/BP_Board.GetCellPositionByNumber` _output_get _playercellnumber))
  (bind _playerpion (`/Game/OldProject/Blueprint/BP_Gameinstance.GetPlayerPionByPlayerId` _as_bp_gameinstance PlayerId))
  ;[1 1 1] Fais spawn l'actor puis le met dans une liste de pion
  (bind _returnvalue_2 (`|SpawnActorFromClass` _playerpion (`KismetMathLibrary.MakeTransform` _celllocation) "Undefined" "MultiplyWithRoot" null null))
  (`KismetArrayLibrary.Array_Add` (`self.PionPlayer`) _returnvalue_2))

(fn `UserConstructionScript`)